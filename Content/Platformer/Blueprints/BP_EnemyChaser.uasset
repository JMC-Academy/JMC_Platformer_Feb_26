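; Chasing enemy for a platformer that hurts the player on contact and can be defeated through its hit zone.
; While the player overlaps DetectionZone, Tick rotates it toward the player on XY and moves it straight at them.
; Capsule hits damage the player and knock them back along the enemy's velocity.
; Leaving HitZone launches the player and reduces enemy health; at zero, it scatters random coins and destroys itself.
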(event `self.ReceiveBeginPlay`
  ; Get Player Reference
  (bind _asbp_third_person_character (cast `/Game/Platformer/Blueprints/BP_ThirdPersonCharacter` (`GameplayStatics.GetPlayerPawn` 0)))
  (set `self.PlayerReference` _asbp_third_person_character))

(event `self.DetectionZone.OnComponentBeginOverlap`
  (params (OverlappedComponent :type "PrimitiveComponent Object Reference") (OtherActor :type "Actor Object Reference") (OtherComp :type "PrimitiveComponent Object Reference") (OtherBodyIndex :type Integer) (bFromSweep :type Boolean) (SweepResult :type "HitResult Structure (by ref)"))
  ; Check if detecting player
  (if (== OtherActor (`self.PlayerReference`))
    (set `self.CanDetectPlayer` true)))

(event `self.DetectionZone.OnComponentEndOverlap`
  (params (OverlappedComponent :type "PrimitiveComponent Object Reference") (OtherActor :type "Actor Object Reference") (OtherComp :type "PrimitiveComponent Object Reference") (OtherBodyIndex :type Integer))
  ; Check if detecting player
  (if (== OtherActor (`self.PlayerReference`))
    (set `self.CanDetectPlayer` false)))

(event `self.ReceiveTick`
  (params (DeltaSeconds :type "Float (single-precision)"))
  (bind (_returnvalue_x _returnvalue_y) (`KismetMathLibrary.BreakVector` (`self.K2_GetActorLocation`)))
  (bind (_returnvalue_x_2 _returnvalue_y_2) (`KismetMathLibrary.BreakVector` (`self.K2_GetActorLocation` (`self.PlayerReference`))))
  ; If player is detected
  (if (`self.CanDetectPlayer`)
    (`|ExecutionSequence`
      (:`then_0`
        ; Look At Player
        (`self.K2_SetActorRotation` (`KismetMathLibrary.FindLookAtRotation` (`KismetMathLibrary.MakeVector` _returnvalue_x _returnvalue_y) (`KismetMathLibrary.MakeVector` _returnvalue_x_2 _returnvalue_y_2))))
      (:`then_1`
        ; Chase player
        (`self.AddMovementInput` (`KismetMathLibrary.Normal` (- (`self.K2_GetActorLocation` (`self.PlayerReference`)) (`self.K2_GetActorLocation`))))))))

(event `self.HitZone.OnComponentEndOverlap`
  (params (OverlappedComponent :type "PrimitiveComponent Object Reference") (OtherActor :type "Actor Object Reference") (OtherComp :type "PrimitiveComponent Object Reference") (OtherBodyIndex :type Integer))
  ; Player hits the enemy hit zone
  (if (== OtherActor (`self.PlayerReference`))
    (`|ExecutionSequence`
      (:`then_0`
        ; Launch Player
        (`self.LaunchCharacter` (`self.PlayerReference`) (`self.LaunchDirection`) false false))
      (:`then_1`
        ; Calculate Enemy Health
        (set `self.Health` (- (`self.Health`) (`self.EnemyDamage`)))
        ; Destroy Enemy
        (if (<= (`self.Health`) 0)
          (`self.LootAndDestroy`))))))

(event `self.CapsuleComponent.OnComponentHit`
  (params (HitComponent :type "PrimitiveComponent Object Reference") (OtherActor :type "Actor Object Reference") (OtherComp :type "PrimitiveComponent Object Reference") (NormalImpulse :type "Vector Structure") (Hit :type "HitResult Structure (by ref)"))
  ; Knockback Effect
  (if (== OtherActor (`self.PlayerReference`))
    (`self.LaunchCharacter` (`self.PlayerReference`) (* (`self.GetVelocity`) (`self.KnockbackStrength`)) false false)
    ; Damage Player
    (`/Game/Platformer/Blueprints/BP_ThirdPersonCharacter.DamagePlayer` (`self.PlayerReference`) (`self.PlayerDamage`))))

(event `LootAndDestroy`
  (bind _returnvalue (`self.GetTransform`))
  ;[0 0.15 0.0576 0.5] Loot And Destroy
  (for _ (range (+ (`KismetMathLibrary.RandomIntegerInRange` 0 (`self.CoinsDropped`)) 1))
    (`|SpawnActorFromClass` "/Game/Platformer/Blueprints/BP_Coin.BP_Coin_C" (`KismetMathLibrary.MakeTransform` (`KismetMathLibrary.MakeVector` (+ (`KismetMathLibrary.RandomFloatInRange` -200.0 200.0) (.x (.location _returnvalue))) (+ (`KismetMathLibrary.RandomFloatInRange` -200.0 200.0) (.y (.location _returnvalue))) (.z (.location _returnvalue))) (.rotation _returnvalue) (.scale _returnvalue)) "Undefined" "MultiplyWithRoot" null null))
  (`self.K2_DestroyActor`))

(fn `UserConstructionScript`)